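; Player component that tracks what the camera is pointing at for the building system.
; Each tick it saves the previous target buildable, then runs a Visibility line trace from the camera along its forward vector, ignoring the player.
; The hit location becomes the target point, and the hit actor, cast to BP_Buildable, becomes the current target buildable.
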(event `self.ReceiveBeginPlay`
  (`|ExecutionSequence`
    (:`then_0`
      ;[1 1 1] Get the player
      (bind _asbp_player (cast `/Game/Assets/Player/BP_Player` (`self.GetOwner`)))
      (set `self.player` _asbp_player))))

(event `self.ReceiveTick`
  (params (DeltaSeconds :type "Float (single-precision)"))
  (bind _c_splayerbuildmanager (`/Game/Assets/Player/BP_Player.C_SPlayerBuildManager` (`self.player`)))
  (`|ExecutionSequence`
    (:`then_0`
      ;[1 1 1] Save the last target building
      (set `C_SPlayerBuildManager.lastTargetBuildable` (`C_SPlayerBuildManager.targetBuildable` _c_splayerbuildmanager) _c_splayerbuildmanager))
    (:`then_1`
      ;[1 1 1] Fill the target information (pointed location, pointed buildable, etc.)
      (`self.FillTargetInformation`))))

(fn `FillTargetInformation`
  (bind _returnvalue (`GameplayStatics.GetPlayerCameraManager` 0))
  (bind _returnvalue_2 (`PlayerCameraManager.GetCameraLocation` _returnvalue))
  (bind _outhit (`KismetSystemLibrary.LineTraceSingle` _returnvalue_2 (+ _returnvalue_2 (* (`Actor.GetActorForwardVector` _returnvalue) 9999.0)) "TraceTypeQuery1" false (`|MakeArray` (`self.player`) :!type "Actor Object Reference")))
  (`|ExecutionSequence`
    (:`then_0`
      (bind (_bblockinghit _binitialoverlap _time _location _impactpoint _normal _impactnormal _physmat _hitactor) (`GameplayStatics.BreakHitResult` _outhit))
      (set `self.targetPoint` _location))
    (:`then_1`
      (bind _asbp_buildable (cast `/Game/Assets/Buildable/BP_Buildable` _hitactor)
        (:`then`
          _)
        (:`CastFailed`
          _))
      (set `C_SPlayerBuildManager.targetBuildable` _asbp_buildable (`/Game/Assets/Player/BP_Player.C_SPlayerBuildManager` (`self.player`))))))