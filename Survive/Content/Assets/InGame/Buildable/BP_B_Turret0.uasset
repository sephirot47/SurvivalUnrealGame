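; Buildable turret actor that manages an on-screen BP_Widget_BuildableHUD with options such as remove and move.
; Each tick it creates or repositions the widget while Building or Pointing Over, and removes it when Built.
; The widget is also removed when the turret sits at world origin or is destroyed.
; Placement projects the actor location to screen and converts it to viewport-normalized anchors centered on the turret.
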(event `self.ReceiveActorBeginOverlap`
  (params (OtherActor :type "Actor Object Reference")))

(event `self.ReceiveTick`
  (params (DeltaSeconds :type "Float (single-precision)"))
  (`|ExecutionSequence`
    (:`then_0`
      (bind _returnvalue (`self.GetCurrentState`))
      (switch `BuildableState` _returnvalue
        (:`Building`
          ;[1 1 1] Handle pointingOver
          ;;[1 1 1] Create the widget if it wasn't created. Othwerise, update its position
          (if (`KismetSystemLibrary.IsValid` (`self.widget`)) :!label _label
            ;;[1 1 1] Update widget position and size
            (`self.UpdateWidgetAnchors`)
            (else
              ;;[1 1 1] Creates the little Widget with the (Remove, Move, etc) and its saved in the "widget" variable
              (`self.CreateAndPositionWidget`))))
        (:`Built`
          ;[1 1 1] If it's not being pointed over anymore, remove the widget, in case it existed
          (`self.RemoveWidget` :!label _label_2))
        (:`PointingOver`
          (goto _label))))
    (:`then_1`
      (if (== (`self.K2_GetActorLocation`) (0.0 0.0 0.0))
        (goto _label_2)))))

(event `self.ReceiveBeginPlay`
  (add `self.OnDestroyed` (delegate `OnDestroyed_Event_0`)))

(event `OnDestroyed_Event_0`
  ;[1 1 1] On destroyed, destroy the widget as well
  (`self.RemoveWidget`))

(fn `CreateAndPositionWidget`
  (bind _returnvalue (`|CreateWidget` "/Game/Assets/InGame/Buildable/BuildableHUD/BP_Widget_BuildableHUD.BP_Widget_BuildableHUD_C"))
  (set `self.widget` _returnvalue)
  (`self.UpdateWidgetAnchors`)
  (`UserWidget.AddToViewport` _returnvalue 0)
  (return))

(fn `GetScreenWidgetPosition`
  (returns (Minimum :type "Vector2D Structure") (Maximum :type "Vector2D Structure"))
  (bind (_x _y) (`KismetMathLibrary.BreakVector2D` (`PlayerController.ProjectWorldLocationToScreen` (`GameplayStatics.GetPlayerController` 0) (`self.K2_GetActorLocation`))))
  ;[1 1 1] Get Minimum
  (bind (_normx _normy) (`self.ScreenNormalized` _x _y))
  ;[1 1 1] Get Maximum
  (bind (_normx_2 _normy_2) (`self.ScreenNormalized` (`self.widgetWidth`) (`self.widgetHeight`)))
  (bind _returnvalue (- (`KismetMathLibrary.MakeVector2D` _normx _normy) (/ (`KismetMathLibrary.MakeVector2D` _normx_2 _normy_2) 2.0)))
  (return _returnvalue (+ _returnvalue (`KismetMathLibrary.MakeVector2D` _normx_2 _normy_2))))

(fn `RemoveWidget`
  (if (`KismetSystemLibrary.IsValid` (`self.widget`))
    (`Widget.RemoveFromParent` (`self.widget`))
    ;[1 1 1] widget = null
    (set `self.widget` null))
  (return))

(fn `UpdateWidgetAnchors`
  (bind (_minimum _maximum) (`self.GetScreenWidgetPosition`))
  (`UserWidget.SetAnchorsInViewport` (`self.widget`) (make `Anchors` _minimum _maximum))
  (return))

(fn `UserConstructionScript`)